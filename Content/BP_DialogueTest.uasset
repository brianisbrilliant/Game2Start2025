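; BP_DialogueTest is a test actor that shows a dialogue widget to a player inside its trigger sphere.
; Sphere overlap greets the character, enables input for that PlayerID's controller and stores the ID; exit disables input and removes the widget.
; E or gamepad left face button creates or reuses W_Dialogue on that player's screen.
; GetNextLine is unfinished, only fetching DT_Dialog's first row.
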(event OnComponentBeginOverlap(Sphere)
  (params (OverlappedComponent :type Primitive%20Component%20Object%20Reference) (OtherActor :type Actor%20Object%20Reference) (OtherComp :type Primitive%20Component%20Object%20Reference) (OtherBodyIndex :type Integer) (bFromSweep :type Boolean) (SweepResult :type Hit%20Result%20Structure%20%28by%20ref%29))
  (bind _asbp_third_person_character (Utilities|Casting|CastToBP_ThirdPersonCharacter OtherActor))
  (Development|PrintString (Utilities|String|Append "Hello player " (Utilities|String|ToString(Integer) (+ (Variables|/Game/ThirdPerson/Blueprints/BP_ThirdPersonCharacter.BP_ThirdPersonCharacter_C|GetPlayerID _asbp_third_person_character) 1)) "!"))
  (Input|EnableInput (Game|GetPlayerController (Variables|/Game/ThirdPerson/Blueprints/BP_ThirdPersonCharacter.BP_ThirdPersonCharacter_C|GetPlayerID _asbp_third_person_character)))
  (Variables|Default|Setlast%20touched%20Player%20ID (Variables|/Game/ThirdPerson/Blueprints/BP_ThirdPersonCharacter.BP_ThirdPersonCharacter_C|GetPlayerID _asbp_third_person_character))
  (Development|PrintString "press E to start dialogue"))

(event OnComponentEndOverlap(Sphere)
  (params (OverlappedComponent :type Primitive%20Component%20Object%20Reference) (OtherActor :type Actor%20Object%20Reference) (OtherComp :type Primitive%20Component%20Object%20Reference) (OtherBodyIndex :type Integer))
  (Utilities|Casting|CastToBP_ThirdPersonCharacter OtherActor)
  (Input|DisableInput (Game|GetPlayerController (Variables|Default|Getlast%20touched%20Player%20ID)))
  (Widget|RemovefromParent (Variables|Default|Getdialog%20widget)) ; remove the widget
)

(event Custom|Get%20Next%20Line
  (bind _outrownames (DataTable|GetDataTableRowNames "/Game/DT_Dialog.DT_Dialog"))
  (bind _returnvalue (Utilities|GetDataTableRow "/Game/DT_Dialog.DT_Dialog" (Utilities|Array|Get(acopy) _outrownames))))

(event EventBeginPlay)

(event Input|KeyboardEvents|DebugKeyE
  (params (Key :type Key%20Structure :default "None") (ActionValue :type Input%20Action%20Value%20Structure))
  ;[0.15 0 0 0.5] Replace this with an input event
  (:Pressed
    (Utilities|IsValid (Variables|Default|Getdialog%20widget) ; Do we already have a dialogue widget?\nThen show that one.\nOtherwise, create a new dialogue widget!
      (:Is%20Valid
        _)
      (:Is%20Not%20Valid
        (bind _returnvalue (UserInterface|CreateWidget "/Game/W_Dialogue.W_Dialogue_C" (Game|GetPlayerController (Variables|Default|Getlast%20touched%20Player%20ID))))
        (Variables|Default|Setdialog%20widget _returnvalue)))
    (UserInterface|Viewport|AddtoPlayerScreen (Variables|Default|Getdialog%20widget))))

(event Input|GamepadEvents|GamepadFaceButtonLeft
  (params (Key :type Key%20Structure :default "None"))
  ;[0.15 0 0 0.5] Replace this with an input event
  (:Pressed
    (Utilities|IsValid (Variables|Default|Getdialog%20widget) ; Do we already have a dialogue widget?\nThen show that one.\nOtherwise, create a new dialogue widget!
      (:Is%20Valid
        _)
      (:Is%20Not%20Valid
        (bind _returnvalue (UserInterface|CreateWidget "/Game/W_Dialogue.W_Dialogue_C" (Game|GetPlayerController (Variables|Default|Getlast%20touched%20Player%20ID))))
        (Variables|Default|Setdialog%20widget _returnvalue)))
    (UserInterface|Viewport|AddtoPlayerScreen (Variables|Default|Getdialog%20widget))))

(fn ConstructionScript)