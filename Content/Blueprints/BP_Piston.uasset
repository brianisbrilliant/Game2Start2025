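; BP_Piston is an animated piston that moves up and down and produces impact feedback for players.
; On BeginPlay a timeline starts, intended to begin at a random time, and lerps the piston's relative height.
; Its Thud event prints a debug message, spawns a randomized-volume and pitch sound (no asset assigned yet), plays force feedback and triggers source-based camera shake for player controllers 0 and 1.
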(event `self.ReceiveBeginPlay`
  (`|ExecutionSequence`
    (:`then_0`
      (bind (_direction _newtrack_0) (`Timeline|Timeline` :`NewTime` (`KismetMathLibrary.RandomFloat`) :!label _label) ; Move the piston up and down\nStart at a random time on beginPlay
        (:`Update`
          (`SceneComponent.K2_SetRelativeLocation` (`self.Piston`) (`KismetMathLibrary.MakeVector` 0.0 0.0 (`KismetMathLibrary.Lerp` -30.0 20.0 _newtrack_0)) false false))
        (:`thud`
          ; Piston Impact
          (`KismetSystemLibrary.PrintString` "Thud")
          (`GameplayStatics.SpawnSoundAtLocation` null (`SceneComponent.K2_GetComponentLocation` (`self.Piston`)) (struct) (`KismetMathLibrary.RandomFloatInRange` 0.0 0.3) (`KismetMathLibrary.RandomFloatInRange` 0.01 0.5) 0.0 null null) ; I don't have any sounds for this yet. Make one!
          (`ForceFeedbackComponent.Play` (`self.ForceFeedback`) 0.0) ; Play Force Feedback for the Controller
          ;; Play Camera Shake from each player.
          (`PlayerController.ClientStartCameraShakeFromSource` (`GameplayStatics.GetPlayerController` 0) "/Game/CS_PistonScreenShake.CS_PistonScreenShake_C" (`self.CameraShakeSource`))
          (`PlayerController.ClientStartCameraShakeFromSource` (`GameplayStatics.GetPlayerController` 1) "/Game/CS_PistonScreenShake.CS_PistonScreenShake_C" (`self.CameraShakeSource`)))))
    (:`then_1`
      (goto _label :!via `SetNewTime`))))

(fn `UserConstructionScript`)